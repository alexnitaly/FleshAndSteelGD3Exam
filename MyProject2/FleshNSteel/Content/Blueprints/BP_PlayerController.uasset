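; Player controller for a card game that sets up the HUD, deck, energy and opening hand on BeginPlay.
; It shows the cursor, creates the main HUD, pads the deck with shuffled generic attack cards and refills energy to maximum.
; DrawUntilFull moves top cards into the hand up to a cap, adding card widgets to the HUD.
; Each widget reads the deck's top after removal, so it receives the following card's data.
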(event Custom|InitializeDeck
  (bind _deck (Variables|Default|GetDeck))
  (while (< (Utilities|Array|LastIndex _deck) 3)
    (Utilities|Array|Add _deck "/Game/Blueprints/CardSystem/Data_Assets/DA_GenericAttack.DA_GenericAttack")
    (Utilities|Array|Shuffle _deck)))

(event Custom|StartTurnResources
  (if (< (Variables|Default|GetCurrentEnergy) (Variables|Default|GetMaxEnergy))
    (Variables|Default|SetCurrentEnergy (Variables|Default|GetMaxEnergy))))

(event EventBeginPlay
  (Variables|Default|SetbShowMouseCursor true)
  (Input|SetInputModeGameandUI 0 0 "LockInFullscreen" true)
  (bind _returnvalue (UserInterface|CreateWidget "/Game/UI/Widget/WBP_MainHUD.WBP_MainHUD_C"))
  (bind _output_get (Variables|Default|SetMainHUDRef _returnvalue))
  (UserInterface|Viewport|AddtoViewport _output_get 0)
  (CallFunction|InitializeDeck)
  (CallFunction|StartTurnResources)
  (CallFunction|DrawUntilFull))

(fn ConstructionScript)

(fn DrawUntilFull
  (bind _deck (Variables|Default|GetDeck))
  (bind _output (Utilities|Array|Get(acopy) _deck))
  (while (and (> (Utilities|Array|Length _deck) 0) (< (Utilities|Array|Length (Variables|Default|GetHand)) 6))
    (Utilities|Array|Add (Variables|Default|GetHand) _output)
    (Utilities|Array|RemoveIndex _deck)
    (bind _returnvalue (UserInterface|CreateWidget "/Game/UI/Widget/WBP_Card.WBP_Card_C" (Game|GetPlayerController 0) _output))
    (Widget|Panel|AddChild (Variables|/Game/UI/Widget/WBP_MainHUD.WBP_MainHUD_C|GetHandContainer (Variables|Default|GetMainHUDRef)) _returnvalue)))