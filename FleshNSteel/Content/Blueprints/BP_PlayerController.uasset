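; Player controller for a card game that sets up the cursor, main HUD, deck, energy and opening hand on BeginPlay.
; InitializeDeck fills and shuffles a deck of generic attack cards, and StartTurnResources tops energy up to maximum.
; DrawUntilFull moves top cards into a capped hand, updating the HUD count and adding card widgets.
; Each widget reads the deck top after removal, so it receives the following card's data.
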(event Custom|InitializeDeck
  (bind _deck (Variables|Default|GetDeck))
  (while (< (Utilities|Array|LastIndex _deck) 10)
    (Utilities|Array|Add _deck "/Game/Blueprints/CardSystem/Data_Assets/DA_GenericAttack.DA_GenericAttack")
    ;[1 1 1] Double dip, making sure the deck counts its size properly
    (Utilities|Array|Shuffle _deck)
    (Default|UpdateDeckCount (Variables|Default|GetMainHUDRef) (Utilities|Array|Length (Variables|Default|GetDeck)))))

(event Custom|StartTurnResources
  (if (< (Variables|Default|GetCurrentEnergy) (Variables|Default|GetMaxEnergy))
    (Variables|Default|SetCurrentEnergy (Variables|Default|GetMaxEnergy))))

(event EventBeginPlay
  (bind _output_get (Variables|Default|SetbShowMouseCursor true))
  (Input|SetInputModeGameandUI (Game|GetPlayerController 0) 0 "LockInFullscreen" _output_get)
  (bind _returnvalue (UserInterface|CreateWidget "/Game/UI/Widget/WBP_MainHUD.WBP_MainHUD_C"))
  (bind _output_get_2 (Variables|Default|SetMainHUDRef _returnvalue))
  (UserInterface|Viewport|AddtoViewport _output_get_2 0)
  (CallFunction|InitializeDeck)
  (CallFunction|StartTurnResources)
  (CallFunction|DrawUntilFull))

(fn ConstructionScript)

(fn DrawUntilFull
  (bind _deck (Variables|Default|GetDeck))
  (bind _output (Utilities|Array|Get(acopy) _deck))
  (while (and (> (Utilities|Array|Length _deck) 0) (< (Utilities|Array|Length (Variables|Default|GetHand)) 5))
    (Utilities|Array|Add (Variables|Default|GetHand) _output)
    (Utilities|Array|RemoveIndex _deck)
    (Default|UpdateDeckCount (Variables|Default|GetMainHUDRef) (Utilities|Array|Length (Variables|Default|GetDeck)))
    (bind _returnvalue (UserInterface|CreateWidget "/Game/UI/Widget/WBP_Card.WBP_Card_C" (Game|GetPlayerController 0) _output))
    (Widget|Panel|AddChild (Variables|/Game/UI/Widget/WBP_MainHUD.WBP_MainHUD_C|GetHandContainer (Variables|Default|GetMainHUDRef)) _returnvalue)))