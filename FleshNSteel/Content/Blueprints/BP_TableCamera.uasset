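; BP_TableCamera is a camera actor that becomes player 0's view target on BeginPlay, intended to add mouse-driven parallax to the view.
; It caches the Camera component's world location as a base.
; Each Tick, it offsets that base along Y and Z by the viewport-centered mouse position scaled by MaxParallax.
; The result is applied to the PlayerController's location, not this actor's; a note flags the follow behavior as needing a fix.
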(event EventBeginPlay
  (Variables|Default|SetBaseLocation (Transformation|GetWorldLocation (Variables|Default|GetCamera)))
  (Game|Player|SetViewTargetwithBlend (Game|GetPlayerController 0) self 0.0 "VTBlend_Linear" 0.0 false))

(event EventTick
  (params (DeltaSeconds :type Float%20%28single-precision%29))
  (bind _returnvalue (Game|GetPlayerController 0))
  (bind _returnvalue_2 (Viewport|GetViewportSize))
  (bind _maxparallax (Variables|Default|GetMaxParallax))
  (bind (_locationx _locationy) (Game|Player|GetMousePosition _returnvalue))
  ;[1 1 1] To Fix: it should follow between the center and the mouse!
  (Transformation|SetActorLocation (Game|GetPlayerController 0) (+ (Math|Vector|MakeVector 0.0 (* (- (/ _locationx (.x _returnvalue_2)) 0.5) _maxparallax) (* (- (/ _locationy (.y _returnvalue_2)) 0.5) _maxparallax)) (Variables|Default|GetBaseLocation)) false false))

(fn ConstructionScript)